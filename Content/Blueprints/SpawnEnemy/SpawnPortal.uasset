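; SpawnPortal is an enemy spawner that starts producing ZombiAI when a ThirdPersonCharacter overlaps its Box trigger.
; If fewer than 50 ZombiAI exist on overlap, it spawns one at the Arrow and repeats every 6 seconds, without rechecking that cap.
; The construction script applies variable-driven transforms to the Box and Arrow.
; Destroying the spawner also destroys its referenced PortalToDestroy.
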(event `self.Box.OnComponentBeginOverlap`
  (params (OverlappedComponent :type "PrimitiveComponent Object Reference") (OtherActor :type "Actor Object Reference") (OtherComp :type "PrimitiveComponent Object Reference") (OtherBodyIndex :type Integer) (bFromSweep :type Boolean) (SweepResult :type "HitResult Structure (by ref)"))
  (bind _arrow (`self.Arrow`))
  (cast `/Game/Blueprints/Character/ThirdPersonCharacter` OtherActor)
  (bind _outactors (`GameplayStatics.GetAllActorsOfClass` "/Game/Blueprints/Enemy/Zombie/ZombiAI.ZombiAI_C"))
  (if (< (`KismetArrayLibrary.Array_Length` _outactors) 50)
    (`AIBlueprintHelperLibrary.SpawnAIFromClass` "/Game/Blueprints/Enemy/Zombie/ZombiAI.ZombiAI_C" null (`SceneComponent.K2_GetComponentLocation` _arrow) (`SceneComponent.K2_GetComponentRotation` _arrow) false null :!label _label)
    (`KismetSystemLibrary.Delay` 6.0)
    (goto _label)))

(event `self.ReceiveDestroyed`
  (`/Game/Blueprints/Interactive/Barricade.Destroy` (`self.Portal to Destroy`)))

(fn `UserConstructionScript`
  (bind _box (`self.Box`))
  (bind _arrow (`self.Arrow`))
  (`SceneComponent.SetRelativeScale3D` _box (`self.Scale`))
  (`SceneComponent.K2_SetRelativeLocation` _box (`self.Location`) false false)
  (`SceneComponent.K2_SetRelativeRotation` _box (`self.Rotation`) false false)
  (`SceneComponent.K2_SetRelativeLocation` _arrow (`self.ArrowLoc`) false false)
  (`SceneComponent.K2_SetRelativeRotation` _arrow (`self.ArrowRot`) false false))