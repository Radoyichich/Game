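; PainVolume is a damage hazard actor that hurts the ThirdPersonCharacter when it begins overlapping.
; Five seconds after play begins, the Moving timeline slides the Cube between StartLocation and EndLocation by lerping its relative location without sweep.
; Each overlap begin casts to the character, sets IsInVolume and calls the character's TakeDamage200 once, with no end-overlap handling.
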(event `self.ReceiveBeginPlay`
  (`KismetSystemLibrary.Delay` 5.0)
  (bind (_direction _newtrack_0) (`Timeline|Moving`)
    (:`Update`
      (`SceneComponent.K2_SetRelativeLocation` (`self.Cube`) (`KismetMathLibrary.VLerp` (`self.Start Location`) (`self.End Location`) _newtrack_0) false false))))

(event `self.ReceiveActorBeginOverlap`
  (params (OtherActor :type "Actor Object Reference"))
  (bind _asthird_person_character (cast `/Game/Blueprints/Character/ThirdPersonCharacter` OtherActor))
  (set `self.IsInVolume?` true)
  (`/Game/Blueprints/Character/ThirdPersonCharacter.TakeDamage200%` _asthird_person_character))

(fn `UserConstructionScript`)