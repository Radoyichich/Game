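; Light puzzle Blueprint that moves a static mesh vertically once its count matches the number of Light actors in the scene.
; Addto increments the counter and compares it with a GetAllActorsOfClass count, while RemoveFrom decrements it, stopping at zero.
; On a match, the TL_Winner timeline plays, adding its track value plus a constant to the mesh's relative Z every update, with sweep.
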(event `Add to`
  ;[1 1 1] Add Until Int = the Amount of Lights are in the Scene
  (set `self.Int` (+ (`self.Int`) 1))
  (bind _outactors (`GameplayStatics.GetAllActorsOfClass` "/Game/Blueprints/Puzzle/Light.Light_C"))
  (if (== (`KismetArrayLibrary.Array_Length` _outactors) (`self.Int`))
    (`self.WinningCondition`)))

(event `WinningCondition`
  (bind (_direction _winner) (`Timeline|TL_Winner`)
    (:`Update`
      (`SceneComponent.K2_AddRelativeLocation` (`self.StaticMesh`) (`KismetMathLibrary.MakeVector` 0.0 0.0 (+ _winner 10.0)) true false))))

(event `RemoveFrom`
  (bind _int (`self.Int`))
  ;[1 1 1] Take Away Int
  (if (> _int 0)
    (set `self.Int` (- _int 1))))

(fn `UserConstructionScript`)