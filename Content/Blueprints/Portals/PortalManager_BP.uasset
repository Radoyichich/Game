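; Portal manager that keeps the views of a linked pair of portals in sync with the player's camera.
; Every tick, two mirrored functions move each portal's PortalView to the camera's transform as seen relative to the opposite portal.
; The remap uses the rotation delta between the portals, with the destination yaw flipped 180 degrees, applied to both camera position and rotation.
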(event `self.ReceiveTick`
  (params (DeltaSeconds :type "Float (single-precision)"))
  (`self.First Portal Update`)
  (`self.Second Portal Update`))

(fn `First Portal Update`
  (bind _defaultsceneroot (`/Game/Blueprints/Portals/FirstPortal_BP.DefaultSceneRoot` (`self.FirstPortal`)))
  (bind _defaultsceneroot_2 (`/Game/Blueprints/Portals/SecondPortal_BP.DefaultSceneRoot` (`self.SecondPortal`)))
  (bind _transformcomponent (`PlayerCameraManager.TransformComponent` (`GameplayStatics.GetPlayerCameraManager` 0)))
  (bind (_returnvalue_roll _returnvalue_pitch _returnvalue_yaw) (`KismetMathLibrary.BreakRotator` (`SceneComponent.K2_GetComponentRotation` _defaultsceneroot_2)))
  (bind _returnvalue (`KismetMathLibrary.NormalizedDeltaRotator` (`KismetMathLibrary.MakeRotator` _returnvalue_roll _returnvalue_pitch (- _returnvalue_yaw 180.0)) (`SceneComponent.K2_GetComponentRotation` _defaultsceneroot)))
  (`SceneComponent.K2_SetWorldLocationAndRotation` (`/Game/Blueprints/Portals/SecondPortal_BP.PortalView` (`self.SecondPortal`)) (+ (- (`SceneComponent.K2_GetComponentLocation` _defaultsceneroot_2) (`KismetMathLibrary.GreaterGreater_VectorRotator` (`SceneComponent.K2_GetComponentLocation` _defaultsceneroot) _returnvalue)) (`KismetMathLibrary.GreaterGreater_VectorRotator` (`SceneComponent.K2_GetComponentLocation` _transformcomponent) _returnvalue)) (`KismetMathLibrary.ComposeRotators` (`SceneComponent.K2_GetComponentRotation` _transformcomponent) _returnvalue) false false))

(fn `Second Portal Update`
  (bind _defaultsceneroot (`/Game/Blueprints/Portals/FirstPortal_BP.DefaultSceneRoot` (`self.FirstPortal`)))
  (bind _defaultsceneroot_2 (`/Game/Blueprints/Portals/SecondPortal_BP.DefaultSceneRoot` (`self.SecondPortal`)))
  (bind _transformcomponent (`PlayerCameraManager.TransformComponent` (`GameplayStatics.GetPlayerCameraManager` 0)))
  (bind (_returnvalue_roll _returnvalue_pitch _returnvalue_yaw) (`KismetMathLibrary.BreakRotator` (`SceneComponent.K2_GetComponentRotation` _defaultsceneroot)))
  (bind _returnvalue (`KismetMathLibrary.NormalizedDeltaRotator` (`KismetMathLibrary.MakeRotator` _returnvalue_roll _returnvalue_pitch (- _returnvalue_yaw 180.0)) (`SceneComponent.K2_GetComponentRotation` _defaultsceneroot_2)))
  (`SceneComponent.K2_SetWorldLocationAndRotation` (`/Game/Blueprints/Portals/FirstPortal_BP.PortalView` (`self.FirstPortal`)) (+ (- (`SceneComponent.K2_GetComponentLocation` _defaultsceneroot) (`KismetMathLibrary.GreaterGreater_VectorRotator` (`SceneComponent.K2_GetComponentLocation` _defaultsceneroot_2) _returnvalue)) (`KismetMathLibrary.GreaterGreater_VectorRotator` (`SceneComponent.K2_GetComponentLocation` _transformcomponent) _returnvalue)) (`KismetMathLibrary.ComposeRotators` (`SceneComponent.K2_GetComponentRotation` _transformcomponent) _returnvalue) false false))

(fn `UserConstructionScript`)