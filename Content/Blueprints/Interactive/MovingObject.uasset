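; A configurable moving platform that travels to an end location while a ThirdPersonCharacter is inside its trigger box and returns when the character leaves.
; Overlap events play or reverse a timeline, with play rate derived from Duration, whose track lerps the platform's relative location from its starting point.
; The construction script applies the mesh, scale and rotation to both the platform and a reference copy positioned at the end location.
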(event `self.ReceiveBeginPlay`
  (set `self.StartLocation` (`SceneComponent.RelativeLocation` (`self.MainPlatform`))))

(event `self.Box.OnComponentBeginOverlap`
  (params (OverlappedComponent :type "PrimitiveComponent Object Reference") (OtherActor :type "Actor Object Reference") (OtherComp :type "PrimitiveComponent Object Reference") (OtherBodyIndex :type Integer) (bFromSweep :type Boolean) (SweepResult :type "HitResult Structure (by ref)"))
  (cast `/Game/Blueprints/Character/ThirdPersonCharacter` OtherActor)
  (`TimelineComponent.SetPlayRate` (`self.MovePlatform`) (/ 1.0 (`self.Duration`)))
  (bind (_direction _movetrack) (`Timeline|MovePlatform` :!label _label)
    (:`Update`
      (`SceneComponent.K2_SetRelativeLocation` (`self.MainPlatform`) (`KismetMathLibrary.VLerp` (`self.StartLocation`) (`self.End Location`) _movetrack) false false))))

(event `self.Box.OnComponentEndOverlap`
  (params (OverlappedComponent :type "PrimitiveComponent Object Reference") (OtherActor :type "Actor Object Reference") (OtherComp :type "PrimitiveComponent Object Reference") (OtherBodyIndex :type Integer))
  (cast `/Game/Blueprints/Character/ThirdPersonCharacter` OtherActor)
  (`TimelineComponent.SetPlayRate` (`self.MovePlatform`) (/ 1.0 (`self.Duration`)))
  (goto _label :!via `Reverse`))

(fn `UserConstructionScript`
  (bind _mainplatform (`self.MainPlatform`))
  (bind _endplatformref (`self.EndPlatformRef`))
  (bind _platformmesh (`self.PlatformMesh`))
  (`StaticMeshComponent.SetStaticMesh` _mainplatform _platformmesh)
  (`StaticMeshComponent.SetStaticMesh` _endplatformref _platformmesh)
  (`SceneComponent.SetRelativeScale3D` _mainplatform (`self.Scale`))
  (`SceneComponent.SetRelativeScale3D` _endplatformref (`self.Scale`))
  (`SceneComponent.K2_SetRelativeRotation` _mainplatform (`self.Rotation`) false false)
  (`SceneComponent.K2_SetRelativeRotation` _endplatformref (`self.Rotation`) false false)
  (`SceneComponent.K2_SetRelativeLocation` _endplatformref (`self.End Location`) false false))