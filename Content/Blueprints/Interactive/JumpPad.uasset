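; Jump pad actor that launches a ThirdPersonCharacter when it overlaps the pad's Box.
; The overlap plays the JumpPadAnimation timeline, which tilts the whole actor's pitch.
; When the timeline finishes, the character jumps, then after a short delay is launched along the Arrow's forward vector scaled by LaunchPower.
; A DoOnce blocks repeat launches until the current one completes.
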(event `self.Box.OnComponentBeginOverlap`
  (params (OverlappedComponent :type "PrimitiveComponent Object Reference") (OtherActor :type "Actor Object Reference") (OtherComp :type "PrimitiveComponent Object Reference") (OtherBodyIndex :type Integer) (bFromSweep :type Boolean) (SweepResult :type "HitResult Structure (by ref)"))
  (bind (_returnvalue_roll _returnvalue_pitch _returnvalue_yaw) (`KismetMathLibrary.BreakRotator` (`self.K2_GetActorRotation`)))
  (bind _asthird_person_character (cast `/Game/Blueprints/Character/ThirdPersonCharacter` OtherActor))
  (bind (_direction _launch_track) (`Timeline|Jump Pad Animation`)
    (:`Update`
      (`self.K2_SetActorRotation` (`KismetMathLibrary.MakeRotator` _returnvalue_roll (`KismetMathLibrary.Lerp` -10.0 10.0 _launch_track) _returnvalue_yaw)))
    (:`Finished`
      (`/Engine/EditorBlueprintResources/StandardMacros.DoOnce` false :!label _label
        (:`Completed`
          (`Character.Jump` _asthird_person_character)
          (`KismetSystemLibrary.Delay` 0.2)
          (`Character.LaunchCharacter` _asthird_person_character (* (`SceneComponent.GetForwardVector` (`self.Arrow`)) (`self.LaunchPower`)) false false)
          (goto _label :!via `Reset`))))))

(fn `UserConstructionScript`)