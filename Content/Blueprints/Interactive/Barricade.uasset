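; Interactive barricade Blueprint that removes itself once a counter of active triggers reaches a required threshold.
; The Destroy event increments SpawnPortalActive, while SwitchDeactivated decrements it.
; Both events then compare the count to SpawnActorDestroyed and destroy the actor if it is equal or higher.
; BeginPlay, overlap, Tick and the construction script are empty, so all behavior relies on those two events being called.
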(event `Destroy`
  (`/Engine/EditorBlueprintResources/StandardMacros.IncrementInt` (`self.SpawnPortalActive`)
    (:`  `
      (if (>= (`self.SpawnPortalActive`) (`self.SpawnActorDestroyed`))
        (`self.K2_DestroyActor` :!label _label)))))

(event `SwitchDeactivated`
  (`/Engine/EditorBlueprintResources/StandardMacros.DecrementInt` (`self.SpawnPortalActive`)
    (:`  `
      (if (>= (`self.SpawnPortalActive`) (`self.SpawnActorDestroyed`))
        (goto _label)))))

(fn `UserConstructionScript`)