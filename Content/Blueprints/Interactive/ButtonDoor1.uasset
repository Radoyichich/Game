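; Interactive door Blueprint that raises its Cube on Activate and returns it to its starting position on Deactivate.
; BeginPlay stores the Cube's world location as the return point.
; The Open timeline lerps from the current location toward a point just above it each update, so upward travel accumulates.
; The Close timeline lerps from the current location back to the stored point, both without sweep.
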(event `self.ReceiveBeginPlay`
  (set `self.InitialLocation` (`SceneComponent.K2_GetComponentLocation` (`self.Cube`))))

(event `/Game/Blueprints/Character/ActivateInterface1.Activate`
  (params (Player :type "Character Object Reference"))
  (bind _returnvalue (`SceneComponent.K2_GetComponentLocation` (`self.Cube`)))
  (bind (_direction _alpha) (`Timeline|Open` :!via `PlayFromStart`)
    (:`Update`
      (`SceneComponent.K2_SetWorldLocation` (`self.Cube`) (`KismetMathLibrary.VLerp` _returnvalue (`KismetMathLibrary.MakeVector` (.x _returnvalue) (.y _returnvalue) (+ (.z _returnvalue) 10.0)) _alpha) false false))))

(event `/Game/Blueprints/Character/ActivateInterface1.Deactivate`
  (params (Player :type "Character Object Reference"))
  (bind (_direction _alpha) (`Timeline|Close` :!via `PlayFromStart`)
    (:`Update`
      (`SceneComponent.K2_SetWorldLocation` (`self.Cube`) (`KismetMathLibrary.VLerp` (`SceneComponent.K2_GetComponentLocation` (`self.Cube`)) (`self.InitialLocation`) _alpha) false false))))

(fn `UserConstructionScript`)