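; Interactive sliding door that moves between two positions using physics rather than animation.
; A physics constraint's linear drive target on X is picked from the Closed flag at BeginPlay, which also sets the door to world origin.
; Each Use event sets the target from the current flag, wakes the door's rigid body, then flips Closed, so the first Use repeats the BeginPlay target.
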(event `self.ReceiveBeginPlay`
  (`SceneComponent.K2_SetWorldLocation` (`self.Door`) (0.0 0.0 0.0) false false)
  (`PhysicsConstraintComponent.SetLinearPositionTarget` (`self.PC_DoorSlide`) (`KismetMathLibrary.MakeVector` (`KismetMathLibrary.SelectFloat` 135.0 -150.0 (`self.Closed`)))))

(event `/Game/Blueprints/Character/Use.Use`
  (`PhysicsConstraintComponent.SetLinearPositionTarget` (`self.PC_DoorSlide`) (`KismetMathLibrary.MakeVector` (`KismetMathLibrary.SelectFloat` 135.0 -150.0 (`self.Closed`))))
  (`PrimitiveComponent.WakeRigidBody` (`self.Door`) "None")
  (set `self.Closed` (not (`self.Closed`))))

(fn `UserConstructionScript`)