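; Interactive switch actor that a ThirdPersonCharacter toggles on and off to drive a list of linked objects.
; Interact waits an activation delay, flips Status and sends ActivateMessage or DeactivateMessage with the player to each ActivatedObject.
; An IsInteracting flag blocks repeat use until the reset delay ends.
; The construction script places an Arrow from PlayerTransform; the node that would move the player's capsule to it is unconnected.
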(event `/Game/Blueprints/Character/InteractInterface.Interact`
  (params (Player :type "Character Object Reference"))
  (bind _activatedobject (`self.ActivatedObject`))
  (bind _player (`self.Player`))
  (bind _asthird_person_character (cast `/Game/Blueprints/Character/ThirdPersonCharacter` Player))
  (set `self.Player` _asthird_person_character)
  (if (not (`self.IsInteracting`))
    (set `self.IsInteracting` true)
    (`KismetSystemLibrary.Delay` (`self.WaitForActivate`))
    (if (== (`self.Status`) 0)
      (set `self.Status` 1)
      (for _array_element _activatedobject
        (message `/Game/Blueprints/Character/ActivateInterface1.Activate` _array_element _player))
      (else
        (set `self.Status` 0)
        (for _array_element_2 _activatedobject
          (message `/Game/Blueprints/Character/ActivateInterface1.Deactivate` _array_element_2 _player))))
    (`KismetSystemLibrary.Delay` (`self.WaitForReset`))
    (set `self.IsInteracting` false)))

(fn `UserConstructionScript`
  (`SceneComponent.K2_SetRelativeTransform` (`self.Arrow`) (`self.PlayerTransform`) false false))